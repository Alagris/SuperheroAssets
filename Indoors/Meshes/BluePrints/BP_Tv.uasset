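; BP_Tv is a wall TV that the player switches off and on with the E key while nearby.
; Overlapping its Box enables input for player controller 0 and opens a Gate, and leaving disables input without closing the Gate.
; Each press passes the Gate into a FlipFlop that swaps the screen material slot between dark plastic and the TV screen, starting with dark.
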(event OnComponentBeginOverlap(Box)
  (params (OverlappedComponent :type Primitive%20Component%20Object%20Reference) (OtherActor :type Actor%20Object%20Reference) (OtherComp :type Primitive%20Component%20Object%20Reference) (OtherBodyIndex :type Integer) (bFromSweep :type Boolean) (SweepResult :type Hit%20Result%20Structure%20%28by%20ref%29))
  (Input|EnableInput (Game|GetPlayerController 0))
  (Utilities|FlowControl|Gate true) ; enters at Open
)

(event OnComponentEndOverlap(Box)
  (params (OverlappedComponent :type Primitive%20Component%20Object%20Reference) (OtherActor :type Actor%20Object%20Reference) (OtherComp :type Primitive%20Component%20Object%20Reference) (OtherBodyIndex :type Integer))
  (Input|DisableInput (Game|GetPlayerController 0)))

(event Input|KeyboardEvents|E
  (params (Key :type Key%20Structure))
  (:Pressed
    (Utilities|FlowControl|Gate true
      (:Exit
        (Utilities|FlowControl|FlipFlop
          (:A
            (Rendering|Material|SetMaterial (Variables|Default|GetSm_WallTv) 2 "/Game/Indoors/Mat/MI_PlasticShinyDark.MI_PlasticShinyDark"))
          (:B
            (Rendering|Material|SetMaterial (Variables|Default|GetSm_WallTv) 2 "/Game/Indoors/Mat/MI_TVscreen.MI_TVscreen")))))))

(fn ConstructionScript)